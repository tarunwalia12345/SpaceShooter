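; Base pickup actor that drifts along the world Y axis and homes in on the player once they come within range.
; A Box overlap serves as the homing radius, storing the first overlapping bpPlayer as the target.
; Each Tick sets ProjectileMovement velocity to DefaultSpeed along Y without a target, or blends it toward the player at IncreasedSpeed using a fixed-alpha, frame-rate-dependent lerp.
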(event `self.ReceiveTick`
  (params (DeltaSeconds :type "Float (single-precision)"))
  (bind _projectilemovement (`self.ProjectileMovement`))
  ;[1 1 1] Movement control
  (`/Engine/EditorBlueprintResources/StandardMacros.IsValid` (`self.bpPlayer`)
    (:`Is Valid`
      (set `MovementComponent.Velocity` (`KismetMathLibrary.VLerp` (`MovementComponent.Velocity` (`self.ProjectileMovement`)) (* (`KismetMathLibrary.Normal` (- (`self.K2_GetActorLocation` (`self.bpPlayer`)) (`self.K2_GetActorLocation`))) (`self.IncreasedSpeed`)) 0.1) _projectilemovement))
    (:`Is Not Valid`
      (set `MovementComponent.Velocity` (`KismetMathLibrary.MakeVector` 0.0 (`self.DefaultSpeed`)) _projectilemovement))))

(event `self.Box.OnComponentBeginOverlap`
  (params (OverlappedComponent :type "PrimitiveComponent Object Reference") (OtherActor :type "Actor Object Reference") (OtherComp :type "PrimitiveComponent Object Reference") (OtherBodyIndex :type Integer) (bFromSweep :type Boolean) (SweepResult :type "HitResult Structure (by ref)"))
  ;[1 1 1] Homing Radius Control
  (bind _asbp_player (cast `/Game/Blueprints/Misc/bpPlayer` OtherActor))
  (`/Engine/EditorBlueprintResources/StandardMacros.IsValid` (`self.bpPlayer`)
    (:`Is Not Valid`
      (set `self.bpPlayer` _asbp_player))))

(fn `UserConstructionScript`)